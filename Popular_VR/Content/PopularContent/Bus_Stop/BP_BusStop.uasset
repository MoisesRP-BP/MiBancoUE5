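; Bus stop actor that fast-travels the player between two hard-coded map locations.
; An overlap box, placed by the construction script from a PortalTransform variable, shows or hides interaction text as the player enters or leaves.
; The Teleport event, not called within this graph, adds a black-screen widget, waits briefly, then moves and rotates the player based on Locations.
; BeginPlay also opens a tutorial video source on VideoPlayer.
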(event OnComponentBeginOverlap(Action_Box)
  (params (OverlappedComponent :type Primitive%20Component%20Object%20Reference) (OtherActor :type Actor%20Object%20Reference) (OtherComp :type Primitive%20Component%20Object%20Reference) (OtherBodyIndex :type Integer) (bFromSweep :type Boolean) (SweepResult :type Hit%20Result%20Structure%20%28by%20ref%29))
  (if (== OtherActor (Game|GetPlayerCharacter 0))
    (Development|SetHiddeninGame (Variables|Default|GetInteraction_Text) false false)))

(event OnComponentEndOverlap(Action_Box)
  (params (OverlappedComponent :type Primitive%20Component%20Object%20Reference) (OtherActor :type Actor%20Object%20Reference) (OtherComp :type Primitive%20Component%20Object%20Reference) (OtherBodyIndex :type Integer))
  (if (== OtherActor (Game|GetPlayerCharacter 0))
    (Development|SetHiddeninGame (Variables|Default|GetInteraction_Text) true false)))

(event EventBeginPlay
  (Media|MediaPlayer|OpenSource (Variables|Default|GetVideoPlayer) "/Game/Movies/tutorial_retirar.tutorial_retirar"))

(event Collision|EventActorBeginOverlap
  (params (OtherActor :type Actor%20Object%20Reference)))

(event EventTick
  (params (DeltaSeconds :type Float%20%28single-precision%29)))

(event EventTeleport
  (bind _returnvalue (Game|GetPlayerCharacter 0))
  (bind _returnvalue_2 (Game|GetPlayerCharacter 0))
  (bind _returnvalue_3 (Game|ConstructObjectfromClass "/Game/PopularContent/NPC/BlackScreenPop.BlackScreenPop_C"))
  (UserInterface|Viewport|AddtoViewport _returnvalue_3 0)
  (Utilities|FlowControl|Delay 0.2)
  (if (== (Variables|Default|GetLocations) 1)
    (Transformation|SetActorLocation _returnvalue "-3770.000000,540.000000,-10.000000" false false)
    (Transformation|SetActorRelativeRotation _returnvalue "0,180.000000, 0")
    (else
      (Transformation|SetActorLocation _returnvalue_2 "430.000000,250.000000,-10.000000" false false)
      (Transformation|SetActorRelativeRotation _returnvalue_2 "0,180.000000, 0"))))

(fn ConstructionScript
  (Transformation|SetRelativeTransform (Variables|Default|GetAction_Box) (Variables|Default|GetPortalTransform) false false))